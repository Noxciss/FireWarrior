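; Base weapon Blueprint that handles firing, reloading and magazine ammo, with debug prints for each attempt.
; Fire_Event spends magazine ammo, plays gun and arms montages, spawns a first-person projectile at the muzzle and plays a sound.
; Reload_Event moves reserve ammo into the magazine immediately as the montages start, without waiting for them to finish.
; A separate AnimateReload graph plays a hard-coded rifle grenade montage on the gun mesh.
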(event Custom|Reload_Event
  (bind _reloadanimation (Variables|Default|GetReloadAnimation))
  (bind _armsreloadanimation (Variables|Default|GetArmsReloadAnimation))
  (Development|PrintString "Try Reload Weapon")
  ;[1 1 1] Check Ammo
  (if (and (> (Variables|Default|GetAmmo) 0) (< (Variables|Default|GetMagazineAmmo) (Variables|Default|GetMagazineSize)))
    (Development|PrintString "Reloading")
    ;[1 1 1] Animate Reload
    (Utilities|FlowControl|Sequence
      (:then_0
        (if (Utilities|IsValid _reloadanimation)
          (Animation|Montage|MontagePlay (Components|SkeletalMesh|GetAnimInstance (Variables|Default|GetGunMesh)) _reloadanimation 1.0 "MontageLength" 0.0 true))
        ;[1 1 1] Set Ammo and Magazine
        (if (> (Variables|Default|GetAmmo) (- (Variables|Default|GetMagazineSize) (Variables|Default|GetMagazineAmmo)))
          (Variables|Default|SetAmmo (- (Variables|Default|GetAmmo) (- (Variables|Default|GetMagazineSize) (Variables|Default|GetMagazineAmmo))))
          (Variables|Default|SetMagazineAmmo (Variables|Default|GetMagazineSize))
          (else
            (Variables|Default|SetMagazineAmmo (+ (Variables|Default|GetAmmo) (Variables|Default|GetMagazineAmmo)))
            (Variables|Default|SetAmmo 0))))
      (:then_1
        ;[1 1 1] Animate Arms Reload
        (if (Utilities|IsValid _armsreloadanimation)
          (Animation|Montage|MontagePlay (Components|SkeletalMesh|GetAnimInstance (Variables|Default|GetArmsMesh)) _armsreloadanimation 1.0 "MontageLength" 0.0 true))))
    (else
      (Development|PrintString "Cannot reload"))))

(event Custom|Fire_Event
  (bind _muzzle (Variables|Default|GetMuzzle))
  (bind _fireanimation (Variables|Default|GetFireAnimation))
  (bind _armsfireanimation (Variables|Default|GetArmsFireAnimation))
  (Development|PrintString "Try Shoot")
  ;[1 1 1] Check Ammo
  (if (>= (Variables|Default|GetMagazineAmmo) (Variables|Default|GetAmmoPerShot))
    ;[1 1 1] Consume Ammo
    (Variables|Default|SetMagazineAmmo (- (Variables|Default|GetMagazineAmmo) (Variables|Default|GetAmmoPerShot)))
    ;[1 1 1] Animate Weapon Fire
    (Utilities|FlowControl|Sequence
      (:then_0
        (if (Utilities|IsValid _fireanimation)
          (Animation|Montage|MontagePlay (Components|SkeletalMesh|GetAnimInstance (Variables|Default|GetGunMesh)) _fireanimation 1.0 "MontageLength" 0.0 true))
        ;[1 1 1] SpawnProjectile
        (Game|SpawnActorfromClass "/Game/FirstPersonBP/Blueprints/FirstPersonProjectile.FirstPersonProjectile_C" (Math|Transform|MakeTransform (Transformation|GetWorldLocation _muzzle) (Transformation|GetWorldRotation _muzzle)) "AdjustIfPossibleButDontSpawnIfColliding" 0 0) ; Spawn projectile
        (Audio|PlaySoundatLocation "/Game/FirstPerson/Audio/FirstPersonTemplateWeaponFire02.FirstPersonTemplateWeaponFire02" (Transformation|GetActorLocation) "0, 0, 0" 1.0 1.0 0.0 0 0 0) ; Play firing sound
      )
      (:then_1
        ;[1 1 1] Animate Arms Fire
        (if (Utilities|IsValid _armsfireanimation)
          (Animation|Montage|MontagePlay (Components|SkeletalMesh|GetAnimInstance (Variables|Default|GetArmsMesh)) _armsfireanimation 1.0 "MontageLength" 0.0 true))))
    (else
      (Development|PrintString "Must Reload"))))

(fn ConstructionScript)